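; Grease pencil Blueprint that feeds procedurally generated placeholder stroke points to a Niagara system.
; SetPlaceholderValues runs on construction and BeginPlay, rebuilding parallel arrays of positions, stroke IDs, point IDs, radii and colors.
; Points form a helix along X, split into gapped strokes every 50 points, with cosine-varied width and red-to-blue color.
; The arrays reach Niagara through array data-interface overrides, alongside a ScreenSpace toggle.
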(event `self.ReceiveBeginPlay`
  (`self.SetPlaceholderValues`))

(fn `SetPlaceholderValues`
  (`|ExecutionSequence`
    (:`then_0`
      (`KismetArrayLibrary.Array_Clear` (`self.PointsPositions`))
      (`KismetArrayLibrary.Array_Clear` (`self.PointsStrokeIDs`))
      (`KismetArrayLibrary.Array_Clear` (`self.PointsRadius`))
      (`KismetArrayLibrary.Array_Clear` (`self.PointsIDs`))
      (`KismetArrayLibrary.Array_Clear` (`self.PointsColors`)))
    (:`then_1`
      (for _index (range (+ (`self.NumPoints`) 1))
        (`|ExecutionSequence`
          (:`then_0`
            (`KismetArrayLibrary.Array_Add` (`self.PointsIDs`) _index))
          (:`then_1`
            (bind _returnvalue (* (/ _index 50) 10))
            (bind _returnvalue_2 (* _index 0.1))
            (`KismetArrayLibrary.Array_Add` (`self.PointsPositions`) (`KismetMathLibrary.MakeVector` (`KismetMathLibrary.Conv_IntToDouble` (+ _index _returnvalue)) (* (`KismetMathLibrary.Sin` _returnvalue_2) 50.0) (* (`KismetMathLibrary.Cos` _returnvalue_2) 50.0))))
          (:`then_2`
            (`KismetArrayLibrary.Array_Add` (`self.PointsStrokeIDs`) _returnvalue))
          (:`then_3`
            (bind _returnvalue_3 (`KismetMathLibrary.MapRangeUnclamped` (`KismetMathLibrary.Cos` (`KismetMathLibrary.Conv_IntToDouble` _index)) -1.0 1.0 0.0 1.0))
            (`KismetArrayLibrary.Array_Add` (`self.PointsRadius`) (`KismetMathLibrary.Lerp` 5.0 8.0 _returnvalue_3)))
          (:`then_4`
            (`KismetArrayLibrary.Array_Add` (`self.PointsColors`) (`KismetMathLibrary.LinearColorLerp` (struct :`R` 1.0 :`A` 1.0) (struct :`B` 1.0 :`A` 0.41) _returnvalue_3))))))
    (:`then_2`
      (`NiagaraDataInterfaceArrayFunctionLibrary.SetNiagaraArrayVector` (`self.Niagara`) "ParticleArray" (`self.PointsPositions`))
      (`NiagaraDataInterfaceArrayFunctionLibrary.SetNiagaraArrayInt32` (`self.Niagara`) "StrokeIDs" (`self.PointsStrokeIDs`))
      (`NiagaraDataInterfaceArrayFunctionLibrary.SetNiagaraArrayInt32` (`self.Niagara`) "IDs" (`self.PointsIDs`))
      (`NiagaraDataInterfaceArrayFunctionLibrary.SetNiagaraArrayFloat` (`self.Niagara`) "Width" (`self.PointsRadius`))
      (`NiagaraComponent.SetVariableBool` (`self.Niagara`) "ScreenSpace" (`self.bScreenSpace`))
      (`NiagaraDataInterfaceArrayFunctionLibrary.SetNiagaraArrayColor` (`self.Niagara`) "Colors" (`self.PointsColors`)))))

(fn `UserConstructionScript`
  (`self.SetPlaceholderValues`))